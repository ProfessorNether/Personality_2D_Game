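; Paper2D side-scrolling player character with run, idle and fall animations, horizontal movement and jumping.
; Tick selects the flipbook from falling state and velocity, and turns the controller yaw to face the X direction of travel.
; A coin-pickup handler on the sprite's overlap casts the other actor to BP_SpriteCharacter, increments and prints its Coins, then destroys this character itself.
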(event OnComponentBeginOverlap(Sprite)
  (params (OverlappedComponent :type Primitive%20Component%20Object%20Reference) (OtherActor :type Actor%20Object%20Reference) (OtherComp :type Primitive%20Component%20Object%20Reference) (OtherBodyIndex :type Integer) (bFromSweep :type Boolean) (SweepResult :type Hit%20Result%20Structure%20%28by%20ref%29))
  ;[1 1 1] Coin Pickup System HUD
  (bind _asbp_sprite_character (Utilities|Casting|CastToBP_SpriteCharacter OtherActor))
  (bind _output_get (Variables|BP_SpriteCharacter_C|SetCoins _asbp_sprite_character (+ (Variables|BP_SpriteCharacter_C|GetCoins _asbp_sprite_character) 1)))
  (Development|PrintString (Utilities|String|ToString(Integer) _output_get))
  (Actor|DestroyActor))

(event Custom|UpdateAnimation
  (Sprite|SetFlipbook (Variables|Default|GetSprite) (select (AI|Components|NavMovement|IsFalling (Variables|Character|GetCharacterMovement)) "/Game/SunnyLand_Assets/sprites/player/jump/FB_player-fall.FB_player-fall" (select (> (Math|Vector|VectorLength (Variables|/Script/Engine.MovementComponent|GetVelocity (Variables|Character|GetCharacterMovement))) 0.0) "/Game/SunnyLand_Assets/sprites/player/run/PB_player-run.PB_player-run" "/Game/SunnyLand_Assets/sprites/player/idle/FB_player-idle.FB_player-idle"))))

(event Custom|UpdateControlRotation
  (Utilities|IsValid (Pawn|GetController)
    (:Is%20Valid
      (Math|Float|CompareFloat (.X (Class|KismetMathLibrary|BreakVector3f (Variables|/Script/Engine.MovementComponent|GetVelocity (Variables|Character|GetCharacterMovement)))) 0.0
        (:>
          (Pawn|SetControlRotation (Pawn|GetController) (Math|Rotator|MakeRotator 0.0 0.0 0.0)))
        (:<
          (Pawn|SetControlRotation (Pawn|GetController) (Math|Rotator|MakeRotator 0.0 0.0 1.8e+02)))))))

(event EventTick
  (params (DeltaSeconds :type Float%20%28single-precision%29))
  (CallFunction|UpdateAnimation)
  (CallFunction|UpdateControlRotation))

(event Input|ActionEvents|InputActionJump
  (params (Key :type Key%20Structure :default "None"))
  ;[1 1 1] Player Movement
  (:Pressed
    (Character|Jump))
  (:Released
    (Character|StopJumping)))

(event Input|AxisEvents|InputAxisMoveRIght
  (params (AxisValue :type Float%20%28single-precision%29))
  ;[1 1 1] Player Movement
  (Pawn|Input|AddMovementInput "1.000000,0.000000,0.000000" AxisValue false))

(fn ConstructionScript)